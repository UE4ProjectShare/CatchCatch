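; BP_GeneratorSystem spawns player characters for CatchCatch by character ID and player ID.
; Its Spawn function looks up the character class in the game state's character table and spawns it at a random one of the first four PlayerStarts.
; It then registers the new character with both IDs, multicasts the player ID registration and returns the character.
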(fn `Spawn`
  (params (CharacterID :type Integer) (PlayerID :type Integer))
  (returns (Character :type "Character Object Reference"))
  (bind _asbp_catch_catch_game_state (cast `/Game/CatchCatch/BP/BP_CatchCatchGameState` (`GameplayStatics.GetGameState`)))
  (bind (_characterattribute_characterid _characterattribute_charactername _characterattribute_charactericon _characterattribute_characterclass) (break `/Game/CatchCatch/Struct/CharacterStruct` (`/Game/CatchCatch/BP/BP_CatchCatchGameState.GetCharacterTableTemplate` _asbp_catch_catch_game_state CharacterID)))
  (if (`KismetSystemLibrary.IsValidClass` _characterattribute_characterclass)
    (bind _outactors (`GameplayStatics.GetAllActorsOfClass` "/Script/Engine.PlayerStart"))
    (bind (_returnvalue_location _returnvalue_rotation) (`KismetMathLibrary.BreakTransform` (`self.GetTransform` (`|GetArrayItem` _outactors (`KismetMathLibrary.RandomInteger` 4)))))
    (bind _returnvalue (`|SpawnActorFromClass` _characterattribute_characterclass (`KismetMathLibrary.MakeTransform` _returnvalue_location _returnvalue_rotation) "Undefined" "OverrideRootScale" null null))
    (bind _asbp_catch_catch_character (cast `/Game/CatchCatch/BP/Character/Base/BP_CatchCatchCharacter` _returnvalue))
    (`/Game/CatchCatch/BP/Character/Base/BP_CatchCatchCharacter.RegisterCharacter` _asbp_catch_catch_character CharacterID PlayerID)
    (`/Game/CatchCatch/BP/Character/Base/BP_CatchCatchCharacter.MultCastRegisterCharacter` _asbp_catch_catch_character PlayerID)
    (return _asbp_catch_catch_character)))

(fn `UserConstructionScript`)