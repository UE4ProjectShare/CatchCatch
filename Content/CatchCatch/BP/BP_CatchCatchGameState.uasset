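; BP_CatchCatchGameState is the CatchCatch game state, which sets up the player system and serves character attribute lookups.
; On BeginPlay, only the authority spawns a BP_PlayerSystem actor and stores it in the PlayerSystem variable.
; GetCharacterTableTemplate finds a character's attributes by looping over the CharacterAttributeDataTable row names and returning the first row whose ID field matches the requested ID.
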(event `self.ReceiveBeginPlay`
  (`/Engine/EditorBlueprintResources/ActorMacros.Switch Has Authority`
    (:`Authority`
      (bind _returnvalue (`|SpawnActorFromClass` "/Game/CatchCatch/BP/System/BP_PlayerSystem.BP_PlayerSystem_C" (`KismetMathLibrary.MakeTransform` (0.0 0.0 0.0)) "Undefined" "OverrideRootScale" null null))
      (set `self.PlayerSystem` _returnvalue))))

(event `self.ReceiveTick`
  (params (DeltaSeconds :type "Float (single-precision)")))

(fn `GetCharacterTablesTemplate`
  (returns (OutRowNames :type "Array of Name"))
  (bind _outrownames (`DataTableFunctionLibrary.GetDataTableRowNames` "/Game/CatchCatch/DataTable/CharacterAttributeDataTable.CharacterAttributeDataTable"))
  (return _outrownames))

(fn `GetCharacterTableTemplate`
  (params (ID :type Integer))
  (returns (CharacterAttribute :type "/Game/CatchCatch/Struct/CharacterAttribute Structure"))
  (bind _outrownames (`self.GetCharacterTablesTemplate`))
  (for _array_element _outrownames
    (bind _returnvalue (`|GetDataTableRow` "/Game/CatchCatch/DataTable/CharacterAttributeDataTable.CharacterAttributeDataTable" _array_element)
      (:`then`
        (if (== (`.ID_2_BDE50D4C42F29D284582429B7ED80239` (break `/Game/CatchCatch/Struct/CharacterAttribute` _returnvalue)) ID)
          (return _returnvalue))))))

(fn `UserConstructionScript`)